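; BP_Pickable is a pickable actor that shows its name when the player character comes within range.
; Overlap events on a detection sphere, filtered to BP_GrimrockLikeCharacter, toggle the name text's visibility and the IsPickable flag.
; The construction script sizes the sphere from DetectionRange.X, sets and offsets the label from variables, and gives it absolute rotation.
; The file only maintains the flag; it contains no pickup logic.
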(event `self.Sphere.OnComponentBeginOverlap`
  (params (OverlappedComponent :type "PrimitiveComponent Object Reference") (OtherActor :type "Actor Object Reference") (OtherComp :type "PrimitiveComponent Object Reference") (OtherBodyIndex :type Integer) (bFromSweep :type Boolean) (SweepResult :type "HitResult Structure (by ref)"))
  (cast `/Game/BP_GrimrockLikeCharacter` OtherActor)
  (`SceneComponent.SetVisibility` (`self.PickableName`) true false)
  (set `self.IsPickable` true))

(event `self.Sphere.OnComponentEndOverlap`
  (params (OverlappedComponent :type "PrimitiveComponent Object Reference") (OtherActor :type "Actor Object Reference") (OtherComp :type "PrimitiveComponent Object Reference") (OtherBodyIndex :type Integer))
  (cast `/Game/BP_GrimrockLikeCharacter` OtherActor)
  (`SceneComponent.SetVisibility` (`self.PickableName`) false false)
  (set `self.IsPickable` false))

(fn `UserConstructionScript`
  (bind _pickablename (`self.PickableName`))
  (`SceneComponent.SetAbsolute` (`self.PickableName`) false true false)
  (`SphereComponent.SetSphereRadius` (`self.Sphere`) (.x (`self.Detection Range`)) true)
  (`SceneComponent.K2_SetWorldLocation` _pickablename (+ (`self.Text Location`) (`SceneComponent.K2_GetComponentLocation` _pickablename)) false false)
  (`TextRenderComponent.K2_SetText` (`self.PickableName`) (`self.Text`)))