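; BP_Interactive is an actor that highlights itself under the mouse cursor to show whether it is interactable.
; On hover it creates a dynamic PP_Outline material, colors it green or red from the Interactable flag, and assigns it to the player camera's post-process materials.
; Hover also toggles custom depth on the Interactive component for the outline and switches the cursor between crosshairs and grab hand.
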(event `self.ReceiveActorBeginCursorOver`
  (bind _outline (`self.Outline`))
  (bind _returnvalue (`KismetMaterialLibrary.CreateDynamicMaterialInstance` "/Game/outline/PP_Outline.PP_Outline"))
  (set `self.Outline` _returnvalue)
  (set `PlayerController.CurrentMouseCursor` "GrabHand" (`GameplayStatics.GetPlayerController` 0))
  (if (`self.Interactable ?`)
    (`MaterialInstanceDynamic.SetVectorParameterValue` _outline "outlineColor" (struct :`G` 1.0 :`B` 0.049962 :`A` 1.0))
    (else
      (`MaterialInstanceDynamic.SetVectorParameterValue` _outline "outlineColor" (struct :`R` 1.0 :`B` 0.040611 :`A` 1.0))))
  (setmembers `PostProcessSettings` :`StructRef` (`CameraComponent.PostProcessSettings` (`self.GetComponentByClass` (`GameplayStatics.GetPlayerCharacter` 0) "/Script/Engine.CameraComponent")) :`WeightedBlendables` (make `WeightedBlendables` (`|MakeArray` (make `WeightedBlendable` 1.0 _outline))))
  (`PrimitiveComponent.SetRenderCustomDepth` (`self.Interactive`) true))

(event `self.ReceiveActorEndCursorOver`
  (set `PlayerController.CurrentMouseCursor` "Crosshairs" (`GameplayStatics.GetPlayerController` 0))
  (`PrimitiveComponent.SetRenderCustomDepth` (`self.Interactive`) false))

(fn `UserConstructionScript`)