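; BP_Porte is a door that swings open once, with an optional locked state lifted by a key.
; On BeginPlay it is interactable unless flagged closed, and PickedtheKey makes it interactable.
; The open event fires once, disables collision on frame, box and door, then a timeline animates the door's yaw.
; That event does not check the interactable flag itself.
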(event `self.ReceiveBeginPlay`
  (set `self.Interactable ?` (not (`self.Isclosed ?`))))

(event `Porte oucre toi !!!`
  (`/Engine/EditorBlueprintResources/StandardMacros.DoOnce` false
    (:`Completed`
      (`PrimitiveComponent.SetCollisionEnabled` (`self.cadre`) "NoCollision")
      (`PrimitiveComponent.SetCollisionEnabled` (`self.Box`) "NoCollision")
      (`PrimitiveComponent.SetCollisionEnabled` (`self.Interactive`) "NoCollision")
      (bind (_direction _angle) (`Timeline|Ouverture de porte` :!via `PlayFromStart`)
        (:`Update`
          (`SceneComponent.K2_SetRelativeRotation` (`self.Interactive`) (`KismetMathLibrary.MakeRotator` (.roll (`SceneComponent.RelativeRotation` (`self.Interactive`))) (.pitch (`SceneComponent.RelativeRotation` (`self.Interactive`))) _angle) false false))))))

(event `PickedtheKey`
  (set `self.Interactable ?` true))

(fn `UserConstructionScript`)