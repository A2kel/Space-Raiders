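; Mutant character Blueprint with events that move it toward a target actor or a location.
; The actor event stores the Target and uses SimpleMoveToActor, while the location event uses AIMoveTo and resumes pursuit of Target two seconds after success.
; A blocked move only prints a debug message based on distance to Target.
; Tick caches velocity length as Speed; UpdateWalkSpeed is an empty stub.
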(event `Mutant Move To Actor`
  (params (Actor :type "Actor Object Reference"))
  (set `self.Target` Actor)
  (`AIBlueprintHelperLibrary.SimpleMoveToActor` (`self.GetController`) (`self.Target`)))

(event `Mutant move to location`
  (params (Loc :type "Vector Structure"))
  (bind _movementresult (`|AIMoveTo` self Loc null)
    (:`OnSuccess`
      (`KismetSystemLibrary.Delay` 2.0)
      (`self.Mutant Move To Actor` (`self.Target`)))
    (:`OnFail`
      (switch `EPathFollowingResult` _movementresult
        (:`Blocked`
          (if (<= (`self.GetDistanceTo` (`self.Target`) self) 400.0)
            (`KismetSystemLibrary.PrintString` "Le'ts fight puny human")
            (else
              (`KismetSystemLibrary.PrintString` "dunno what happened"))))))))

(event `self.ReceiveBeginPlay`)

(event `self.ReceiveTick`
  (params (DeltaSeconds :type "Float (single-precision)"))
  (set `self.Speed` (`KismetMathLibrary.VSize` (`self.GetVelocity` self))))

(fn `Update_Walk_Speed`)

(fn `UserConstructionScript`)