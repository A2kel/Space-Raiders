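; Mutant pawn that patrols by moving its skeletal mesh along a spline until it is dead.
; The Patrol event sets the speed and opens a gate that lets Tick advance or rewind patrol time, with distance computed as speed times time.
; At spline ends it either loops to the start or pauses briefly and reverses, flipping the mesh's rotation offset for each direction.
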(event `self.ReceiveTick`
  (params (DeltaSeconds :type "Float (single-precision)"))
  (if (not (`self.Mutant Is dead`))
    (`/Engine/EditorBlueprintResources/StandardMacros.Gate` true :!label _label
      (:`Exit`
        (set `self.Delta Time` DeltaSeconds)
        (if (`self.Aller ?`)
          (if (>= (`self.Distance`) (`SplineComponent.GetSplineLength` (`self.Spline`)))
            (if (`self.Loop ?`)
              (set `self.Patrol time` 0.0)
              (set `self.Distance` 0.0)
              (else
                (set `self.Speed` 0.0)
                (`KismetSystemLibrary.Delay` 2.0)
                (set `self.Aller ?` false)
                (set `self.Speed` 120.0)))
            (else
              (set `self.Patrol time` (+ (`self.Patrol time`) (`self.Delta Time`)))
              (set `self.Distance` (* (`self.Speed`) (`self.Patrol time`)))
              (`SceneComponent.K2_SetWorldTransform` (`self.MutantSkel`) (`KismetMathLibrary.MakeTransform` (.location (`SplineComponent.GetTransformAtDistanceAlongSpline` (`self.Spline`) (`self.Distance`) "World" false)) (`KismetMathLibrary.ComposeRotators` (.rotation (`SplineComponent.GetTransformAtDistanceAlongSpline` (`self.Spline`) (`self.Distance`) "World" false)) (struct :`Yaw` -90.0)) (.scale (`SplineComponent.GetTransformAtDistanceAlongSpline` (`self.Spline`) (`self.Distance`) "World" false))) false false)))
          (elif (<= (`self.Distance`) 0.0)
            (set `self.Speed` 0.0)
            (`KismetSystemLibrary.Delay` 2.0)
            (set `self.Aller ?` true)
            (set `self.Speed` 120.0)
            (else
              (set `self.Patrol time` (- (`self.Patrol time`) (`self.Delta Time`)))
              (set `self.Distance` (* (`self.Patrol time`) (`self.Speed`)))
              (`SceneComponent.K2_SetWorldTransform` (`self.MutantSkel`) (`KismetMathLibrary.MakeTransform` (.location (`SplineComponent.GetTransformAtDistanceAlongSpline` (`self.Spline`) (`self.Distance`) "World" false)) (`KismetMathLibrary.ComposeRotators` (.rotation (`SplineComponent.GetTransformAtDistanceAlongSpline` (`self.Spline`) (`self.Distance`) "World" false)) (struct :`Yaw` 90.0)) (.scale (`SplineComponent.GetTransformAtDistanceAlongSpline` (`self.Spline`) (`self.Distance`) "World" false))) false false))))))))

(event `Patrol`
  (set `self.Speed` 120.0)
  (set `self.Aller ?` true)
  (goto _label :!via `Open`))

(fn `UserConstructionScript`)